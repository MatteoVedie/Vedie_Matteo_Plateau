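; Game mode for the memory card mini-game that handles pair matching and scoring.
; On BeginPlay it shows the memory HUD and caches game mode and game instance references.
; OnCardClicked holds the first card, then compares names with the second: matches add both values and are destroyed, mismatches call TurnCard on both.
; When no cards remain, it shows the end screen and adds the score to the player's total in BP_GameInstance.
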(event `self.ReceiveBeginPlay`
  (bind _returnvalue (`|CreateWidget` "/Game/HUD/WB_HUDMINIGAMEMemory.WB_HUDMINIGAMEMemory_C"))
  (`UserWidget.AddToViewport` _returnvalue 0)
  (bind _asbp_game_mode (cast `/Game/BP/BP_GameMode` (`GameplayStatics.GetGameMode`)))
  (set `self.As BP Game Mode` _asbp_game_mode)
  (bind _asbp_game_instance (cast `/Game/BP/BP_GameInstance` (`GameplayStatics.GetGameInstance`)))
  (set `self.As BP Game Instance` _asbp_game_instance))

(fn `OnCardClicked`
  (params (Card :type "/Game/BP/MiniJeuMemoire/BP_Card Object Reference"))
  (bind _as_bp_game_instance (`self.As BP Game Instance`))
  (bind _player_id (`self.Player Id`))
  (if (`KismetSystemLibrary.IsValid` (`self.PrevCard`))
    (if (`|EnumEquality` (`/Game/BP/MiniJeuMemoire/BP_Card.Name` Card) (`/Game/BP/MiniJeuMemoire/BP_Card.Name` (`self.PrevCard`)))
      (set `self.Score` (+ (+ (`/Game/BP/MiniJeuMemoire/BP_Card.Value` Card) (`/Game/BP/MiniJeuMemoire/BP_Card.Value` (`self.PrevCard`))) (`self.Score`)))
      (`self.K2_DestroyActor` Card)
      (`self.K2_DestroyActor` (`self.PrevCard`))
      (set `self.NbrOfCardAlive` (- (`self.NbrOfCardAlive`) 2))
      (else
        (`/Game/BP/MiniJeuMemoire/BP_Card.TurnCard` Card)
        (`/Game/BP/MiniJeuMemoire/BP_Card.TurnCard` (`self.PrevCard`))))
    (set `self.PrevCard` null)
    (if (== (`self.NbrOfCardAlive`) 0)
      (bind _returnvalue (`|CreateWidget` "/Game/HUD/WB_FinMiniGame.WB_FinMiniGame_C"))
      (`UserWidget.AddToViewport` _returnvalue 0)
      (bind _playerscore (`/Game/BP/BP_GameInstance.GetPlayerScoreByPlayerId` _as_bp_game_instance _player_id))
      (`/Game/BP/BP_GameInstance.SetPlayerScoreByPlayerId` _as_bp_game_instance _player_id (+ _playerscore (`self.Score`))))
    (else
      (set `self.PrevCard` Card))))

(fn `UserConstructionScript`)