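; Game mode for a board game that spawns player 0's pawn piece and a dice, and handles a roll-and-move turn.
; BeginPlay reads the saved cell number from BP_GameInstance and, after a short delay, spawns BP_Pion at that Board cell's position, then spawns BP_Dice.
; RollDiceAndMore rolls the dice, adds the result to the stored cell number and moves the piece to the matching cell.
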(event `self.ReceiveBeginPlay`
  (bind _asbp_game_instance (cast `/Game/BP/BP_GameInstance` (`GameplayStatics.GetGameInstance`)))
  (bind _output_get (set `self.As Game Instance` _asbp_game_instance))
  (bind _player_cell_number (`/Game/BP/BP_GameInstance.GetPlayerCellNumberByPlayerId` _output_get 0))
  (`KismetSystemLibrary.Delay` 0.2)
  (bind _celllocations (`/Game/BP/BP_Board.GetCellPositionsByNumber` (`self.Board`) _player_cell_number))
  (bind _returnvalue (`|SpawnActorFromClass` "/Game/BP/BP_Pion.BP_Pion_C" (`KismetMathLibrary.Conv_VectorToTransform` _celllocations) "Undefined" "MultiplyWithRoot" null null))
  (set `self.PionPlayer1` _returnvalue)
  (bind _returnvalue_2 (`|SpawnActorFromClass` "/Game/BP/BP_Dice.BP_Dice_C" (`KismetMathLibrary.MakeTransform` (0.0 0.0 0.0)) "Undefined" "MultiplyWithRoot" null null))
  (set `self.Dice` _returnvalue_2))

(fn `RollDiceAndMore`
  (bind _as_game_instance (`self.As Game Instance`))
  (bind _dice (`self.Dice`))
  (`/Game/BP/BP_Dice.RollDice` _dice)
  (bind _player_cell_number (`/Game/BP/BP_GameInstance.GetPlayerCellNumberByPlayerId` _as_game_instance 0))
  (bind _returnvalue (+ _player_cell_number (`/Game/BP/BP_Dice.ActualDiceResult` _dice)))
  (`/Game/BP/BP_GameInstance.SetPlayerCellNumberByPlayerId` _as_game_instance 0 _returnvalue)
  (bind _celllocations (`/Game/BP/BP_Board.GetCellPositionsByNumber` (`self.Board`) _returnvalue))
  (`/Game/BP/BP_Pion.MoveToNewCell` (`self.PionPlayer1`) _celllocations))

(fn `UserConstructionScript`)