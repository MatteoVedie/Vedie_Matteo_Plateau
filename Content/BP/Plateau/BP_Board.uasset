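; BP_Board is the game board, holding the list of cells that players occupy.
; On BeginPlay it registers itself on BP_GameMode as the Board and caches the number of cells in ListCell.
; It exposes that cell count and looks up a player's socket position on a cell by index, delegating to that cell's GetSocketPosByPlayerId.
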(event `self.ReceiveBeginPlay`
  (bind _asbp_game_mode (cast `/Game/BP/BP_GameMode` (`GameplayStatics.GetGameMode`)))
  (bind _output_get (set `self.As BP Game Mode` _asbp_game_mode))
  (bind _output_get_2 (set `/Game/BP/BP_GameMode.Board` self _output_get))
  (set `self.CaseNumber` (`KismetArrayLibrary.Array_Length` (`/Game/BP/Plateau/BP_Board.ListCell` _output_get_2))))

(fn `GetCellNumber`
  (returns (`Cell Number` :type Integer))
  (return (`self.CaseNumber`)))

(fn `GetCellPositionsByNumber`
  (params (`Cell Index` :type Integer) (PlayerId :type Integer))
  (returns (CellLocations :type "Vector Structure"))
  (bind _socketpos (`/Game/BP/Plateau/BP_Cell.GetSocketPosByPlayerId` (`|GetArrayItem` (`self.ListCell`) `Cell Index`) PlayerId))
  (return _socketpos))

(fn `UserConstructionScript`)