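; Board cell Blueprint that ends the game and announces the winner when its Action runs.
; It caches BP_GameInstance on BeginPlay and extends the parent cell's Action.
; The Action shows the WB_Fin widget, compares the scores of players 0 and 1 from the game instance, and sets a French winner label.
; A tie is announced as a Player 2 win.
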(event `self.ReceiveBeginPlay`
  (`parent.ReceiveBeginPlay`)
  (bind _asbp_game_instance (cast `/Game/BP/BP_GameInstance` (`GameplayStatics.GetGameInstance`)))
  (set `self.As BP Game Instance_0` _asbp_game_instance))

(fn `Action`
  (params (`Player Id` :type Integer))
  (bind _as_bp_game_instance_0 (`self.As BP Game Instance_0`))
  (`parent.Action` `Player Id`)
  (bind _returnvalue (`|CreateWidget` "/Game/HUD/WB_Fin.WB_Fin_C"))
  (`UserWidget.AddToViewport` _returnvalue 0)
  (bind _playerscore (`/Game/BP/BP_GameInstance.GetPlayerScoreByPlayerId` _as_bp_game_instance_0 0))
  (bind _playerscore_2 (`/Game/BP/BP_GameInstance.GetPlayerScoreByPlayerId` _as_bp_game_instance_0 1))
  (if (> _playerscore _playerscore_2)
    (`/Game/HUD/WB_Fin.ChangeTextFin` _returnvalue "Joueur 1 !")
    (else
      (`/Game/HUD/WB_Fin.ChangeTextFin` _returnvalue "Joueur 2 !"))))

(fn `UserConstructionScript`
  (`parent.UserConstructionScript`))