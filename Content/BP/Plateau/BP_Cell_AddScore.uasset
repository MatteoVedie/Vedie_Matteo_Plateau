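; Board cell (Plateau) actor that awards a fixed score bonus to a player when its action runs.
; It overrides Action, calls the parent version, then reads that player's score from BPGameInstance by PlayerId and writes it back increased by a hardcoded amount.
; A debug print shows the bonus, and the event graph holds only disabled default events.
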(fn `Action`
  (params (`Player Id` :type Integer))
  (`parent.Action` `Player Id`)
  (bind _playerscore (`/Game/BP/BP_GameInstance.GetPlayerScoreByPlayerId` (`self.As BP Game Instance`) `Player Id`))
  (`/Game/BP/BP_GameInstance.SetPlayerScoreByPlayerId` (`self.As BP Game Instance`) `Player Id` (+ _playerscore 5))
  (`KismetSystemLibrary.PrintString` "5"))

(fn `UserConstructionScript`
  (`parent.UserConstructionScript`))