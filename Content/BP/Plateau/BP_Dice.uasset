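; BP_Dice is a Blueprint that rolls a configurable set of dice for the game.
; On BeginPlay it caches a reference to BP_GameMode.
; RollDice spawns one BP_D actor per die at the world origin.
; Each loop pass overwrites ActualDiceResult with a random integer between the dice count and count times die type, so the total is uniformly random rather than a sum of individual rolls.
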(event `self.ReceiveBeginPlay`
  (bind _asbp_game_mode (cast `/Game/BP/BP_GameMode` (`GameplayStatics.GetGameMode`)))
  (set `self.As BP Game Mode` _asbp_game_mode))

(fn `RollDice`
  (bind _dicenumber (`self.DiceNumber`))
  (set `self.ActualDiceResult` (`self.ActualDiceResult`))
  (for _ (range 1 (+ (`self.DiceNumber`) 1))
    (`|SpawnActorFromClass` "/Game/BP/Plateau/BP_D.BP_D_C" (`KismetMathLibrary.MakeTransform` (0.0 0.0 0.0)) "Undefined" "MultiplyWithRoot" null null)
    (set `self.ActualDiceResult` (`KismetMathLibrary.RandomIntegerInRange` _dicenumber (* _dicenumber (`self.DiceType`))))))

(fn `UserConstructionScript`)