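; BP_D is a die actor whose rolled face is read from six directional components: Top, Behind, Down, Right, Left and Front.
; ShowDResult finds the first component whose forward vector exactly equals world up, with zero tolerance, and stores its one-based index in NotActualDResult.
; IsStopped compares the actor's location across a four-second delay to detect rest, but the branch is empty and never triggers ShowDResult.
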(event `IsStopped`
  (set `self.DLocation` (`self.K2_GetActorLocation`))
  (`KismetSystemLibrary.Delay` 4.0)
  (if (== (`self.DLocation`) (`self.K2_GetActorLocation`))
    _))

(event `ShowDResult`
  (for (_array_element _array_index) (`|MakeArray` (`self.Top`) (`self.Behind`) (`self.Down`) (`self.Right`) (`self.Left`) (`self.Front`))
    (if (== (`SceneComponent.GetForwardVector` _array_element) (0.0 0.0 1.0))
      (break)))
  (set `self.NotActualDResult` (+ _array_index 1)))

(fn `UserConstructionScript`)