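; BP_Dice is a dice-rolling Blueprint that rolls once when play begins.
; RollDice resets ActualDiceResult, then adds one random integer for each of DiceNumber dice.
; Each roll ranges from zero to DiceType inclusive, so zero is a possible result.
; The running total prints on screen in red after every die rather than only at the end.
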(event `self.ReceiveBeginPlay`
  (`self.RollDice`))

(fn `RollDice`
  (set `self.ActualDiceResult` 0)
  (for _ (range 1 (+ (`self.DiceNumber`) 1))
    (bind _output_get (set `self.ActualDiceResult` (+ (`self.ActualDiceResult`) (`KismetMathLibrary.RandomIntegerInRange` 0 (`self.DiceType`)))))
    (`KismetSystemLibrary.PrintString` (`KismetStringLibrary.Conv_IntToString` _output_get) true true (struct :`R` 1.0 :`G` 0.022075 :`A` 1.0))))

(fn `UserConstructionScript`)